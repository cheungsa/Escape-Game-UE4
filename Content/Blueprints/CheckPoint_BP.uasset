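; Checkpoint actor that records the player's position and offers a Space-bar teleport while the player is inside it.
; Box overlap by a DefaultPawn writes location and rotation to a CheckpointSaveGame in Slot1, creating it if absent.
; Only when updating an existing save does it also copy the transform to the LoadLevel game instance.
; Overlap enables input; Space teleports the pawn to a hard-coded spot, and teleporting or leaving disables input.
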(event `self.Box.OnComponentBeginOverlap`
  (params (OverlappedComponent :type "PrimitiveComponent Object Reference") (OtherActor :type "Actor Object Reference") (OtherComp :type "PrimitiveComponent Object Reference") (OtherBodyIndex :type Integer) (bFromSweep :type Boolean) (SweepResult :type "HitResult Structure (by ref)"))
  (bind _location (`self.Location`))
  (bind _saversubclass (`self.SaverSubClass`))
  (bind _rotation (`self.Rotation`))
  ;[1 1 1] Logging player's location and rotation
  (bind _asdefault_pawn (cast `DefaultPawn` OtherActor))
  (bind _output_get (set `self.Location` (`self.K2_GetActorLocation` _asdefault_pawn)))
  (`KismetSystemLibrary.PrintString` (`KismetStringLibrary.Conv_VectorToString` _output_get))
  (bind _output_get_2 (set `self.Rotation` (`self.K2_GetActorRotation` _asdefault_pawn)))
  (`KismetSystemLibrary.PrintString` (`KismetStringLibrary.Conv_RotatorToString` _output_get_2))
  ;[1 1 1] Open Maze game
  (`self.EnableInput` (`GameplayStatics.GetPlayerController` 0))
  (bind _returnvalue (`GameplayStatics.DoesSaveGameExist` "Slot1"))
  (if _returnvalue
    (bind _returnvalue_2 (`GameplayStatics.LoadGameFromSlot` "Slot1"))
    (bind _output_get_3 (set `self.SaverSubClass` _returnvalue_2))
    (bind _ascheckpoint_save_game (cast `/Game/Blueprints/CheckpointSaveGame` _output_get_3))
    (set `/Game/Blueprints/CheckpointSaveGame.LastRotation` _rotation _ascheckpoint_save_game)
    (bind _output_get_4 (set `/Game/Blueprints/CheckpointSaveGame.LastLocation` _location _ascheckpoint_save_game))
    (bind _returnvalue_3 (`GameplayStatics.SaveGameToSlot` _saversubclass "Slot1"))
    (`KismetSystemLibrary.PrintString` (`KismetStringLibrary.Conv_BoolToString` _returnvalue_3))
    (bind _asload_level (cast `/Game/Blueprints/LoadLevel` (`GameplayStatics.GetGameInstance`)))
    (set `/Game/Blueprints/LoadLevel.PlayerLocation` _output_get_4 _asload_level)
    (set `/Game/Blueprints/LoadLevel.PlayerRotation` _rotation _asload_level)
    (else
      (bind _returnvalue_4 (`GameplayStatics.CreateSaveGameObject` "/Game/Blueprints/CheckpointSaveGame.CheckpointSaveGame_C"))
      (bind _output_get_5 (set `self.SaverSubClass` _returnvalue_4))
      (bind _ascheckpoint_save_game_2 (cast `/Game/Blueprints/CheckpointSaveGame` _output_get_5))
      (set `/Game/Blueprints/CheckpointSaveGame.LastRotation` _rotation _ascheckpoint_save_game_2)
      (set `/Game/Blueprints/CheckpointSaveGame.LastLocation` _location _ascheckpoint_save_game_2)
      (bind _returnvalue_5 (`GameplayStatics.SaveGameToSlot` _saversubclass "Slot1"))
      (`KismetSystemLibrary.PrintString` (`KismetStringLibrary.Conv_BoolToString` _returnvalue_5)))))

(event `Key|SpaceBar`
  (params (Key :type "Key Structure"))
  ;[1 1 1] Open Maze game
  (:`Pressed`
    (`KismetSystemLibrary.PrintString` "Teleporting")
    (`self.K2_TeleportTo` :`self` (`Controller.K2_GetPawn` (`GameplayStatics.GetPlayerController` 0)) :`DestLocation` (-795.0 -1623.0 127.158691))
    (`self.DisableInput` null)))

(event `self.ReceiveActorEndOverlap`
  (params (OtherActor :type "Actor Object Reference"))
  (`self.DisableInput` null))

(fn `UserConstructionScript`)