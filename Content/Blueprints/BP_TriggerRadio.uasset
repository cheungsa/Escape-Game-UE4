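; BP_TriggerRadio is a radio trigger that plays a "Mary Had a Little Lamb" nursery rhyme on a key press.
; Overlap begin and end enable and disable input on the actor, with no check on the overlapping actor and no PlayerController passed.
; Pressing 4 prints a debug message and plays the sound at the actor's location.
; The PlayerController casts are leftover nodes that never run.
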(event `self.ReceiveActorBeginOverlap`
  (params (OtherActor :type "Actor Object Reference"))
  (`self.EnableInput` null))

(event `Key|Four`
  (params (Key :type "Key Structure"))
  (:`Pressed`
    (`KismetSystemLibrary.PrintString` "Pressed 4 key")
    (`GameplayStatics.PlaySoundAtLocation` "/Game/Audio/Mary_Had_a_Little_Lamb__Nursery_Rhyme__Kids_Songs_Animation_for_Children.Mary_Had_a_Little_Lamb__Nursery_Rhyme__Kids_Songs_Animation_for_Children" (`self.K2_GetActorLocation`))))

(event `self.ReceiveActorEndOverlap`
  (params (OtherActor :type "Actor Object Reference"))
  (`self.DisableInput` null))

(fn `UserConstructionScript`)