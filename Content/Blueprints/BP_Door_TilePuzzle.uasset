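; Door actor for a tile puzzle, apparently meant to swing open once nine tiles are lit.
; The PuzzleOverlap event loops over the TilePuzzle array, adds each lit tile to NumTileLitUp and prints a debug message.
; The count check, door rotation and counter reset are not connected, so the door never rotates and the count accumulates across calls.
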(event `self.ReceiveTick`
  (params (DeltaSeconds :type "Float (single-precision)")))

(event `PuzzleOverlap`
  (for _array_element (`self.TilePuzzle`)
    (if (`/Game/Blueprints/BP_PuzzleBoard.IsOn` _array_element)
      (set `self.NumTileLitUp` (+ (`self.NumTileLitUp`) 1))))
  (`KismetSystemLibrary.PrintString` "completed loop"))

(fn `UserConstructionScript`)