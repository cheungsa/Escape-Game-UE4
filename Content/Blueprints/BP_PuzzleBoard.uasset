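; BP_PuzzleBoard is a single pad in a Lights Out-style tile puzzle linked to a door.
; When an actor of the player pawn's class enters its Box, it flips its own IsOn state and that of every pad in AdjacentPads.
; It then calls PuzzleOverlap on the TileDoor, cast to BP_Door_TilePuzzle, and prints a debug string.
; Tick sets the Cube's on or off material from IsOn every frame.
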(event `self.ReceiveBeginPlay`)

(event `self.ReceiveActorBeginOverlap`
  (params (OtherActor :type "Actor Object Reference")))

(event `self.ReceiveTick`
  (params (DeltaSeconds :type "Float (single-precision)"))
  (bind _cube (`self.Cube`))
  (if (`self.IsOn`)
    (`PrimitiveComponent.SetMaterial` _cube 0 "/Game/Materials/M_IsOn.M_IsOn")
    (else
      (`PrimitiveComponent.SetMaterial` _cube 0 "/Game/Materials/M_IsOff.M_IsOff"))))

(event `self.Box.OnComponentBeginOverlap`
  (params (OverlappedComponent :type "PrimitiveComponent Object Reference") (OtherActor :type "Actor Object Reference") (OtherComp :type "PrimitiveComponent Object Reference") (OtherBodyIndex :type Integer) (bFromSweep :type Boolean) (SweepResult :type "HitResult Structure (by ref)"))
  (if (== (`GameplayStatics.GetObjectClass` OtherActor) (`GameplayStatics.GetObjectClass` (`Controller.K2_GetPawn` (`GameplayStatics.GetPlayerController` 0))))
    (if (`self.IsOn`)
      (set `self.IsOn` false)
      (else
        (set `self.IsOn` true)))
    (for _array_element (`self.AdjacentPads`)
      (if (`/Game/Blueprints/BP_PuzzleBoard.IsOn` _array_element)
        (set `/Game/Blueprints/BP_PuzzleBoard.IsOn` false _array_element)
        (else
          (set `/Game/Blueprints/BP_PuzzleBoard.IsOn` true _array_element))))
    (bind _asbp_door_tile_puzzle (cast `/Game/Blueprints/BP_Door_TilePuzzle` (`self.TileDoor`)))
    (`/Game/Blueprints/BP_Door_TilePuzzle.PuzzleOverlap` _asbp_door_tile_puzzle)
    (`KismetSystemLibrary.PrintString` "calling event")))

(fn `UserConstructionScript`)