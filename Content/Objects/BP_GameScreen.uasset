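; BP_GameScreen is a world object that shows a floating name label when the player comes near.
; The construction script fills its TextRender from the ObjectName variable.
; Each Tick it measures the distance to the controlled pawn, showing the label turned toward the pawn within a short radius.
; Outside that radius it hides the label and disables the actor's input; nothing in these graphs enables it.
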(event `self.ReceiveTick`
  (params (DeltaSeconds :type "Float (single-precision)"))
  (bind _textrender (`self.TextRender`))
  (if (< (`KismetMathLibrary.VSize` (- (`self.K2_GetActorLocation` (`Controller.K2_GetPawn` (`GameplayStatics.GetPlayerController` 0))) (`self.K2_GetActorLocation`))) 250.0)
    (`SceneComponent.SetVisibility` _textrender true false)
    (`SceneComponent.K2_SetWorldRotation` (`self.TextRender`) (`KismetMathLibrary.FindLookAtRotation` (`self.K2_GetActorLocation`) (`self.K2_GetActorLocation` (`Controller.K2_GetPawn` (`GameplayStatics.GetPlayerController` 0)))) false false)
    (else
      (`SceneComponent.SetVisibility` _textrender false false)
      (`self.DisableInput` (`GameplayStatics.GetPlayerController` 0)))))

(fn `UserConstructionScript`
  (`TextRenderComponent.K2_SetText` (`self.TextRender`) (`self.ObjectName`)))